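; Player pawn that coordinates wind turbine spawning, placement and energy preview.
; When spawning starts, it feeds the HUD's spawn location to the TurbineSpawner component.
; On each placement change, a complex line trace from TurbinePlacer samples the windmap through the BP_Ground found at BeginPlay.
; That value updates the selected turbine's previewed energy and windmap value, then the preview-change notification is raised.
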(event OnSpawnStart(TurbineSpawner)
  (params (Turbine :type Turbine%20Object%20Reference))
  ;[0.01764 0.01764 0.01764] Set Spawn Position for Turbine
  (bind _asbp_hud (Utilities|Casting|CastToBP_HUD (HUD|GetHUD (Game|GetPlayerController 0))))
  (bind _worldposition (Default|GetSpawnLocation _asbp_hud))
  (Variables|/Script/WindEnergyIdle_CPP.TurbineSpawner|SetSpawnLocation (Variables|Default|GetTurbineSpawner) _worldposition))

(event OnPlacementChange(TurbinePlacer)
  (params (Turbine :type Turbine%20Object%20Reference))
  ;[0.006995 0.006995 0.006995] OnPlacementChange
  (CallFunction|GetWindmapValue))

(event EventBeginPlay
  (|CallParentFunction)
  ;[0 0 0] Get Reference To Ground
  (bind _returnvalue (Actor|GetActorOfClass "/Game/Blueprints/BP_Ground.BP_Ground_C"))
  (Variables|Default|SetGround _returnvalue))

(fn ConstructionScript)

(fn GetWindmapValue
  (bind _turbineplacer (Variables|Default|GetTurbinePlacer))
  (bind _turbineselector (Variables|Default|GetTurbineSelector))
  (bind _returnvalue (Class|TurbineSelector|GetSelectedTurbine _turbineselector))
  (if (Class|TurbinePlacer|IsPlacing _turbineplacer)
    (bind _outhit (Collision|LineTraceByChannel (Class|TurbinePlacer|GetWorldLocation _turbineplacer) (* (Class|TurbinePlacer|GetWorldDirection _turbineplacer) 1e+06) "TraceTypeQuery3" true 0 "None"))
    (bind _returnvalue_2 (Class|Ground|GetWindMapValue (Variables|Default|GetGround) _outhit))
    (Class|TurbineEnergyController|SetPreviewedEnergy (Variables|/Script/WindEnergyIdle_CPP.Turbine|GetTurbineEnergyController _returnvalue) _returnvalue_2)
    (Class|Turbine|SetWindMapValue _returnvalue _returnvalue_2)
    (Default|CallOnPreviewEnergyChange _returnvalue)))