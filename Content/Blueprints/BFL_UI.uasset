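; UI Blueprint function library that formats money and energy amounts as short, suffixed display values.
; GetMoneyText and GetEnergyText repeatedly divide by 1000 to pick a Postfixs entry, stopping at the last one, then append it to the value shown with two decimals.
; A separate DoubleToString helper floors a value to two decimal places before converting it to a string.
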(fn GetMoneyText
  (params (Money :type Float%20%28double-precision%29))
  (bind _output_get (LocalVariables|SetConvertedMoney Money))
  (while (and (>= _output_get 1e+03) (< (LocalVariables|GetExponent) (- (Utilities|Array|Length (LocalVariables|GetPostfixs)) 1)))
    ;[1 1 1] Loop Body
    (LocalVariables|SetDecimal (Math|Float|%(Float) (LocalVariables|GetConvertedMoney) 1e+03))
    (LocalVariables|SetConvertedMoney (/ (LocalVariables|GetConvertedMoney) 1e+03))
    (LocalVariables|SetExponent (+ (LocalVariables|GetExponent) 1)))
  (return (Utilities|Text|ToText(String) (Utilities|String|Append (Utilities|String|ToString(Text) (Utilities|Text|ToText(Float) (LocalVariables|GetConvertedMoney) "HalfToEven" false true 1 3 2 2)) (Utilities|Array|Get(acopy) (LocalVariables|GetPostfixs) (LocalVariables|GetExponent))))))

(fn DoubletoString
  (params (InputValue :type Float%20%28double-precision%29))
  (return (Utilities|String|ToString(Float) (/ (Math|Conversions|ToFloat(Integer) (Math|Float|Floor (* InputValue 1e+02))) 1e+02))))

(fn GetEnergyText
  (params (Energy :type Float%20%28double-precision%29))
  (bind _output_get (LocalVariables|SetConvertedEnergyPerSecond Energy))
  (while (and (>= _output_get 1e+03) (< (LocalVariables|GetExponent) (- (Utilities|Array|Length (LocalVariables|GetPostfixs)) 1)))
    ;[1 1 1] Loop Body
    (LocalVariables|SetConvertedEnergyPerSecond (/ (LocalVariables|GetConvertedEnergyPerSecond) 1e+03))
    (LocalVariables|SetExponent (+ (LocalVariables|GetExponent) 1)))
  (return (Utilities|Text|ToText(String) (Utilities|String|Append (Utilities|String|Append (Utilities|String|ToString(Text) (Utilities|Text|ToText(Float) (LocalVariables|GetConvertedEnergyPerSecond) "HalfToEven" false true 1 3 2 2)) " ") (Utilities|Array|Get(acopy) (LocalVariables|GetPostfixs) (LocalVariables|GetExponent))))))