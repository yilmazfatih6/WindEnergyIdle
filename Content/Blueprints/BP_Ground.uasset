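; Ground Blueprint that exposes a wind multiplier for any hit point on its surface, based on the Windmap texture in its mesh material.
; On BeginPlay it copies that texture into a helper material instance and draws it to a render target, making the map readable from Blueprint.
; GetWindMapValue converts a hit's collision UV to a pixel, reads it and remaps its HSV brightness to a multiplier with a nonzero floor.
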(event EventBeginPlay
  (bind _rendertarget (Variables|Default|GetRenderTarget))
  ;[1 0.2633 0.9574] Create Dynamic Material Instance
  (bind _returnvalue (Rendering|Material|CreateDynamicMaterialInstance (Rendering|Material|GetMaterial (Variables|Default|GetStaticMeshComponent) 0) "None" "None" :!class /Script/Engine.KismetMaterialLibrary))
  (Variables|Default|SetMaterialInstance _returnvalue)
  ;[0.2172 0.2027 1] Create Temp Dynamic Material Instance
  (bind _returnvalue_2 (Rendering|Material|CreateDynamicMaterialInstance (Variables|Default|GetMaterialWindmap) "None" "None" :!class /Script/Engine.KismetMaterialLibrary))
  (Variables|Default|SetMaterialWindmapInstance _returnvalue_2)
  ;[0 1 0.9702] Assign Windmap Material To Windmap Material Instance
  (bind _returnvalue_3 (Rendering|Material|GetTextureParameterValue (Variables|Default|GetMaterialInstance) "Windmap" :!class /Script/Engine.MaterialInstanceDynamic))
  (Rendering|Material|SetTextureParameterValue (Variables|Default|GetMaterialWindmapInstance) "Windmap" _returnvalue_3)
  ;[1 0 0] Draw Material To Render Target
  (Rendering|ClearRenderTarget2D _rendertarget)
  (Rendering|DrawMaterialtoRenderTarget _rendertarget (Variables|Default|GetMaterialWindmapInstance)))

(fn ConstructionScript)

(fn GetWindMapValue
  (params (HitResult :type Hit%20Result%20Structure))
  (bind (_uv _returnvalue) (Class|GameplayStatics|FindCollisionUV HitResult))
  (bind _rendertarget (Variables|Default|GetRenderTarget))
  (bind (_x _y) (Math|Vector2D|BreakVector2D _uv))
  (Utilities|Casting|CastToStaticMeshComponent (.HitComponent (Collision|BreakHitResult HitResult)))
  (if _returnvalue
    (bind _returnvalue_2 (Class|KismetRenderingLibrary|ReadRenderTargetPixel (Variables|Default|GetRenderTarget) (Math|Float|Truncate (* (Variables|/Script/Engine.TextureRenderTarget2D|GetSizeX _rendertarget) _x)) (Math|Float|Truncate (* (Variables|/Script/Engine.TextureRenderTarget2D|GetSizeY _rendertarget) _y))))
    (return (Math|Float|Lerp 0.1 1.0 (.V (Math|Color|RGBtoHSV(LinearColor) (Math|Conversions|ToLinearColor(Color) _returnvalue_2)))))
    (else
      (Development|PrintString "Couldn't find UV" true true "(R=0.000000,G=0.660000,B=1.000000,A=1.000000)" 0.1))))