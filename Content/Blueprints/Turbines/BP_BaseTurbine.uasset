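; BP_BaseTurbine is a turbine Blueprint that, by its name, serves as the base for turbine actors.
; Its capsule component forwards begin and end overlap events, with the other actor, to BeginOverlap and EndOverlap, which are defined outside this file.
; GetEnergyTextPosition exposes the world transform of the EnergyTextPosition component.
; The construction script is empty, and a debug overlap print is left unconnected.
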(event OnComponentBeginOverlap(CapsuleComponent)
  (params (OverlappedComponent :type Primitive%20Component%20Object%20Reference) (OtherActor :type Actor%20Object%20Reference) (OtherComp :type Primitive%20Component%20Object%20Reference) (OtherBodyIndex :type Integer) (bFromSweep :type Boolean) (SweepResult :type Hit%20Result%20Structure%20%28by%20ref%29))
  ;[0.06667 1 0] Begin Overlap - Capsule
  (Class|Turbine|BeginOverlap OtherActor))

(event OnComponentEndOverlap(CapsuleComponent)
  (params (OverlappedComponent :type Primitive%20Component%20Object%20Reference) (OtherActor :type Actor%20Object%20Reference) (OtherComp :type Primitive%20Component%20Object%20Reference) (OtherBodyIndex :type Integer))
  ;[0.06667 1 0] End Overlap - Capsule
  (Class|Turbine|EndOverlap OtherActor))

(fn ConstructionScript)

(fn GetEnergyTextPosition
  (return (Transformation|GetWorldTransform (Variables|Default|GetEnergyTextPosition))))