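; BP_BaseTurbine is a base turbine actor with a rotating propeller and a selection mesh.
; On BeginPlay it assigns SMSelection as the SelectionMesh and points the RotatingMovement component at the Propeller, so only that part spins.
; Capsule begin and end overlap events forward the other actor to BeginOverlap and EndOverlap, whose logic is defined outside these graphs.
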(event OnComponentBeginOverlap(Capsule)
  (params (OverlappedComponent :type Primitive%20Component%20Object%20Reference) (OtherActor :type Actor%20Object%20Reference) (OtherComp :type Primitive%20Component%20Object%20Reference) (OtherBodyIndex :type Integer) (bFromSweep :type Boolean) (SweepResult :type Hit%20Result%20Structure%20%28by%20ref%29))
  ;[0.06667 1 0] Begin Overlap - Capsule
  (Class|BaseTurbine|BeginOverlap OtherActor))

(event OnComponentEndOverlap(Capsule)
  (params (OverlappedComponent :type Primitive%20Component%20Object%20Reference) (OtherActor :type Actor%20Object%20Reference) (OtherComp :type Primitive%20Component%20Object%20Reference) (OtherBodyIndex :type Integer))
  ;[0.06667 1 0] End Overlap - Capsule
  (Class|BaseTurbine|EndOverlap OtherActor))

(event EventBeginPlay
  ;[1 1 1] BeginPlay
  (Variables|Default|SetSelectionMesh (Variables|Default|GetSM_Selection))
  (Components|Movement|SetUpdatedComponent (Variables|Default|GetRotatingMovement) (Variables|Default|GetPropeller)))

(event Collision|EventActorBeginOverlap
  (params (OtherActor :type Actor%20Object%20Reference)))

(event EventTick
  (params (DeltaSeconds :type Float%20%28single-precision%29)))

(fn ConstructionScript)