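; Level streamer that loads levels by number from a level list as streamed sublevels, one current level at a time.
; LoadLevel first runs a check that unloads the current level and validates the game instance and level list.
; It then saves the clamped number as the last level, maps it to a list index and streams that soft reference in without blocking.
; UnloadLevel extends the parent's version with a non-blocking stream unload.
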(event EventBeginPlay)

(event Collision|EventActorBeginOverlap
  (params (OtherActor :type Actor%20Object%20Reference)))

(event EventTick
  (params (DeltaSeconds :type Float%20%28single-precision%29)))

(event EventLoadLevel
  (params (LevelNumber :type Integer))
  (bind _returnvalue (Math|Integer|Clamp(Integer) LevelNumber 1 2147483647))
  ;[1 1 1] Load Level
  (|ValidCheck
    (:Is%20Valid
      (Class|DefaultSaveGame|SetLastLevelNumber (Variables|Default|GetDefaultSaveGame) _returnvalue)
      (Development|PrintString (Utilities|String|Append "[BP_LevelStreamer] Level Number = " (Utilities|String|ToString(Integer) _returnvalue)) false)
      (bind _returnvalue_2 (Class|LevelStreamer|GetLevelIndex _returnvalue))
      (Development|PrintString (Utilities|String|Append "[BP_LevelStreamer] Level Index = " (Utilities|String|ToString(Integer) _returnvalue_2)) false)
      (bind _output_get (Variables|Default|SetCurrentLevel (Utilities|Array|Get(acopy) (Variables|/Script/WindEnergyIdle_CPP.LevelListDataAsset|GetLevels (Variables|Default|GetLevelList)) _returnvalue_2)))
      (Class|GameplayStatics|LoadStreamLevelbySoftObjectPtr _output_get true false))))

(event EventUnloadLevel
  ;[1 1 1] Unload Level
  (|CallParentFunction)
  (bind _currentlevel (Variables|Default|GetCurrentLevel)
    (:then
      (Class|GameplayStatics|UnloadStreamLevelbySoftObjectPtr _currentlevel false))
    (:else)))

(fn ConstructionScript)