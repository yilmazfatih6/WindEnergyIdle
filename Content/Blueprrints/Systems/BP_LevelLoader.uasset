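; BP_LevelLoader opens a game level from a requested level number and records it as the last level in the default save game object.
; LoadLevel first runs a Valid Check macro on the game instance, level list and save game.
; It then clamps the number to at least 1, converts it through GetLevelIndex and opens that data asset's level by object reference.
; Debug prints trace each step.
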(event EventLoadLevel
  (params (LevelNumber :type Integer))
  (bind _returnvalue (Math|Integer|Clamp(Integer) LevelNumber 1 2147483647))
  ;[1 1 1] Load Level
  (Development|PrintString (Utilities|String|Append "[BP_LevelLoader] Level Number = " (Utilities|String|ToString(Integer) LevelNumber)) false)
  (|ValidCheck
    (:Is%20Valid
      (Development|PrintString "[BP_LevelLoader] Is valid complete!" false)
      (Class|DefaultSaveGame|SetLastLevelNumber (Variables|Default|GetDefaultSaveGame) _returnvalue)
      (Development|PrintString (Utilities|String|Append "[BP_LevelLoader] Clamped Level Number = " (Utilities|String|ToString(Integer) _returnvalue)) false)
      (bind _returnvalue_2 (Class|LevelLoader|GetLevelIndex _returnvalue))
      (Development|PrintString (Utilities|String|Append "[BP_LevelLoader] Level Index = " (Utilities|String|ToString(Integer) _returnvalue_2)) false)
      (Game|OpenLevel(byObjectReference) (Variables|/Script/WindEnergyIdle_CPP.LevelDataAsset|GetLevel (Utilities|Array|Get(acopy) (Variables|/Script/WindEnergyIdle_CPP.LevelListDataAsset|GetLevelsDataAssets (Variables|Default|GetLevelList)) _returnvalue_2))))))